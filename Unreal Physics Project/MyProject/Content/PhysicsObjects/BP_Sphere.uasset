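; Physics sphere that feeds hand-rolled vector-based collision checks against other spheres and a single plane.
; On BeginPlay it caches the surface normal and PointB location of the first BP_Plane found, then breaks the loop.
; Each Tick it passes centre-to-centre vectors and radii of all PO_Sphere actors to CheckForSphereCollision.
; It also passes the plane-point-to-sphere vector and cached normal to CheckForPlaneCollision.
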(event Custom|BreakFindNormalLoop
  (Utilities|Array|ForEachLoopwithBreak (stale EventBeginPlay _outactors)) ; enters at Break
)

(event EventBeginPlay
  (bind _outactors (Actor|GetAllActorsOfClass "/Game/PhysicsObjects/BP_Plane.BP_Plane_C"))
  (bind _array_element (Utilities|Array|ForEachLoopwithBreak _outactors)
    (:LoopBody
      (Variables|Default|SetPlaneNormal (Variables|/Game/PhysicsObjects/BP_Plane.BP_Plane_C|GetSurfaceNormal _array_element))
      (Variables|Default|SetArbritraryPointK (Transformation|GetWorldLocation (Variables|/Game/PhysicsObjects/BP_Plane.BP_Plane_C|GetPointB _array_element)))
      (CallFunction|BreakFindNormalLoop))))

(event EventTick
  (params (DeltaSeconds :type Float%20%28single-precision%29))
  (bind _outactors (Actor|GetAllActorsOfClass "/Script/MyProject.PO_Sphere"))
  (for _array_element _outactors
    ;[1 1 1] Sphere to sphere detection
    (Class|POSphere|CheckforSphereCollision (- (Transformation|GetActorLocation _array_element) (Transformation|GetActorLocation)) (Variables|/Script/MyProject.PO_Sphere|GetmRadius _array_element)))
  (Class|POSphere|CheckforPlaneCollision (- (Transformation|GetActorLocation) (Variables|Default|GetArbritraryPointK)) (Variables|Default|GetPlaneNormal)))

(fn ConstructionScript)