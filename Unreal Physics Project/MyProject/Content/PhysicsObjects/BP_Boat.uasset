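; BP_Boat is an early-stage boat physics actor that so far only estimates how deep it is submerged.
; Each Tick it stores the delta time and derives a submersed length from its world Z and BaseSideLength, clamped between negative side length and zero.
; The result is only printed to screen for debugging; no buoyancy force or movement is applied.
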(event EventBeginPlay)

(event Collision|EventActorBeginOverlap
  (params (OtherActor :type Actor%20Object%20Reference)))

(event EventTick
  (params (DeltaSeconds :type Float%20%28single-precision%29))
  (bind _basesidelength (Variables|Default|GetBaseSideLength))
  (Variables|Default|Setdt (Utilities|Time|GetWorldDeltaSeconds))
  (bind _output_get (Variables|Default|SetmSubmersedLength (Math|Float|Min(Float) (Math|Float|Max(Float) (+ (+ (.z (Transformation|GetActorLocation)) _basesidelength) (/ _basesidelength 2.0)) (* _basesidelength -1.0)) 0.0)))
  (Development|PrintString (Utilities|String|ToString(Float) _output_get)))

(fn ConstructionScript)