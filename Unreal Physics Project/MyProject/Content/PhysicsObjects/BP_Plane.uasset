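; BP_Plane is a plane physics object that derives its surface normal from three point components, PointA, PointB and PointC.
; On BeginPlay it crosses the world-space vectors from C to A and from B to A, then stores the normalized result in SurfaceNormal.
; The normal is computed only once at startup, and the construction script is empty.
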(event EventBeginPlay
  (bind _pointa (Variables|Default|GetPointA))
  (bind _returnvalue (Transformation|GetWorldLocation _pointa))
  (Variables|Default|SetCA (- _returnvalue (Transformation|GetWorldLocation (Variables|Default|GetPointC))))
  (Variables|Default|SetBA (- _returnvalue (Transformation|GetWorldLocation (Variables|Default|GetPointB))))
  (Variables|Default|SetSurfaceNormal (Math|Vector|Normalize (Math|Vector|CrossProduct (Variables|Default|GetCA) (Variables|Default|GetBA)))))

(fn ConstructionScript)